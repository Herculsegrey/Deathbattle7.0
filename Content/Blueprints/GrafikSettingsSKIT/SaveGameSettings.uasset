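; SaveGameSettings is a data container, apparently a save game object, for the player's graphics settings.
; It stores a command and a setting value for each category: overall graphics, shadows, anti-aliasing, post-processing, textures, distance and effects.
; SetSettings writes all values at once, while ReturnCommands and ReturnEnums read back the commands and the enum settings separately.
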(fn SetSettings
  (params (GraphicsCommand :type String) (ShadowCommand :type String) (AACommand :type String) (PPCommand :type String) (TextureCommand :type String) (DistanceCommand :type String) (EffectCommand :type String) (GraphicSetting :type EGraphicsSettings%20Enum :default "NewEnumerator0") (ShadowSetting :type EGraphicsSettings%20Enum :default "NewEnumerator0") (AASetting :type EGraphicsSettings%20Enum :default "NewEnumerator0") (PPSetting :type EGraphicsSettings%20Enum :default "NewEnumerator0") (TextureSetting :type EGraphicsSettings%20Enum :default "NewEnumerator0") (DistanceSetting :type EGraphicsSettings%20Enum :default "NewEnumerator0") (EffectSetting :type EGraphicsSettings%20Enum :default "NewEnumerator0"))
  (Variables|Default|SetGraphicsCommand GraphicsCommand)
  (Variables|Default|SetShadowCommand ShadowCommand)
  (Variables|Default|SetAACommand AACommand)
  (Variables|Default|SetPPCommand PPCommand)
  (Variables|Default|SetTextureCommand TextureCommand)
  (Variables|Default|SetDistanceCommand DistanceCommand)
  (Variables|Default|SetEffectCommand EffectCommand)
  (Variables|Default|SetGraphicSetting GraphicSetting)
  (Variables|Default|SetShadowSetting ShadowSetting)
  (Variables|Default|SetAASetting AASetting)
  (Variables|Default|SetPPSetting PPSetting)
  (Variables|Default|SetTextureSetting TextureSetting)
  (Variables|Default|SetDistanceSetting DistanceSetting)
  (Variables|Default|SetEffectSetting EffectSetting))

(fn ReturnCommands
  (return (Variables|Default|GetGraphicsCommand) (Variables|Default|GetShadowCommand) (Variables|Default|GetAACommand) (Variables|Default|GetPPCommand) (Variables|Default|GetTextureCommand) (Variables|Default|GetDistanceCommand) (Variables|Default|GetEffectCommand)))

(fn ReturnEnums
  (return (Variables|Default|GetGraphicSetting) (Variables|Default|GetShadowSetting) (Variables|Default|GetAASetting) (Variables|Default|GetPPSetting) (Variables|Default|GetTextureSetting) (Variables|Default|GetDistanceSetting) (Variables|Default|GetEffectSetting)))