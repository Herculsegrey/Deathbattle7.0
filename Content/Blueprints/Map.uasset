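; Map is a damageable actor Blueprint that burns and is removed when its health runs out.
; AnyDamage prints a debug string, then subtracts the damage from MapHealth.
; At zero or below, it spawns a P_Fire emitter at the Destructible component's transform, waits briefly, then destroys itself.
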(event Game|Damage|EventAnyDamage
  (params (Damage :type Float%20%28single-precision%29) (DamageType :type Damage%20Type%20Object%20Reference) (InstigatedBy :type Controller%20Object%20Reference) (DamageCauser :type Actor%20Object%20Reference))
  (bind _destructible (Variables|Default|GetDestructible))
  (bind _returnvalue (Transformation|GetWorldTransform _destructible))
  (Development|PrintString (Utilities|String|Append "took" (Utilities|String|ToString(Float) Damage) "damage from" (Utilities|String|ToString(Float) (Variables|Default|GetMapHealth))))
  (bind _output_get (Variables|Default|SetMapHealth (- (Variables|Default|GetMapHealth) Damage)))
  (if (<= _output_get 0.0)
    ;[1 1 1] Kanske fuckar här
    (Effects|SpawnEmitteratLocation "/Game/StarterContent/Particles/P_Fire.P_Fire" (.location _returnvalue) (.rotation _returnvalue) (.scale _returnvalue))
    (Utilities|FlowControl|Delay 2.5)
    (Actor|DestroyActor)))

(event Input|KeyboardEvents|F
  (params (Key :type Key%20Structure :default "None")))

(fn ConstructionScript)